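; BP_SmallButton is a labeled VR toggle button actor that flips between on and off when a VR hand overlaps it.
; IsVrHand filters overlaps through VRTemplateGameMode, then the toggle plays an on or off sound and passes the new state to ButtonCallback.
; A dynamic material instance is updated every Tick with the button color, glowing only while on, and the construction script sets the label text.
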(event `self.ReceiveBeginPlay`
  (bind _returnvalue (`PrimitiveComponent.CreateDynamicMaterialInstance` (`self.Cube1`) 0 "/Game/MyMaterials/SmallButton.SmallButton" "None"))
  (set `self.MaterialInstance` _returnvalue))

(event `self.ReceiveActorBeginOverlap`
  (params (OtherActor :type "Actor Object Reference"))
  (bind _asvrtemplate_game_mode (cast `/Game/SjolieVRTemplates/VRTemplateGameMode` (`GameplayStatics.GetGameMode`)))
  (bind _result (`/Game/SjolieVRTemplates/VRTemplateGameMode.IsVRHand` _asvrtemplate_game_mode OtherActor))
  (if _result
    (bind _output_get (set `self.TurnedOn` (not (`self.TurnedOn`))))
    (`GameplayStatics.PlaySoundAtLocation` (select `bool` _output_get :`false` "/Game/Sounds/ButtonOff.ButtonOff" :`true` "/Game/Sounds/ButtonOn.ButtonOn" :!type "SoundBase Object Reference") (`self.K2_GetActorLocation`) (struct) 1.0 1.0 0.0 null null null)
    (`/Game/BPActors/Logic/BoolCallback.Callback` (`self.ButtonCallback`) (`self.TurnedOn`))))

(event `self.ReceiveTick`
  (params (DeltaSeconds :type "Float (single-precision)"))
  (bind _buttoncolor (`self.ButtonColor`))
  (`MaterialInstanceDynamic.SetVectorParameterValue` (`self.MaterialInstance`) "Color" _buttoncolor)
  (`MaterialInstanceDynamic.SetVectorParameterValue` (`self.MaterialInstance`) "EmissiveColor" (select `bool` (`self.TurnedOn`) :`true` _buttoncolor)))

(fn `UserConstructionScript`
  (`TextRenderComponent.K2_SetText` (`self.Label`) (`self.LabelText`)))