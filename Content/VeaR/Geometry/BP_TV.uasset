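; BP_TV is a television prop whose screen can be switched on and off.
; The construction script creates a dynamic material instance on the Screen component, and BeginPlay caches its ScreenBrightness parameter as the default.
; TurnOff sets that brightness to zero and TurnOn restores the cached value, each updating the IsOn flag.
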(event `self.ReceiveBeginPlay`
  (bind _returnvalue (`MaterialInstanceDynamic.K2_GetScalarParameterValue` (`self.materialInstance`) "ScreenBrightness"))
  (set `self.defaultBrightness` _returnvalue))

(event `TurnOff`
  (`MaterialInstanceDynamic.SetScalarParameterValue` (`self.materialInstance`) "ScreenBrightness" 0.0)
  (set `self.isOn` false))

(event `TurnOn`
  (`MaterialInstanceDynamic.SetScalarParameterValue` (`self.materialInstance`) "ScreenBrightness" (`self.defaultBrightness`))
  (set `self.isOn` true))

(fn `UserConstructionScript`
  (bind _returnvalue (`PrimitiveComponent.CreateDynamicMaterialInstance` (`self.Screen`) 0 null "None"))
  (set `self.materialInstance` _returnvalue))