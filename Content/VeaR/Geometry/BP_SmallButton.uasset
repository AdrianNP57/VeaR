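; BP_SmallButton is a labeled VR toggle button that a hand flips on overlap.
; IsVrHand filters overlaps through VRTemplateGameMode; a valid touch inverts TurnedOn, plays an on or off sound, and notifies ButtonCallback.
; Tick drives a dynamic material's color and emissive glow from that state and copies TurnedOn to an optional Clone button.
; The construction script applies the label text.
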(event `self.ReceiveBeginPlay`
  ;[1 1 1] Create material instance
  (bind _returnvalue (`PrimitiveComponent.CreateDynamicMaterialInstance` (`self.Cube1`) 0 "/Game/MyMaterials/SmallButton.SmallButton" "None"))
  (set `self.MaterialInstance` _returnvalue))

(event `self.ReceiveActorBeginOverlap`
  (params (OtherActor :type "Actor Object Reference"))
  ;[1 1 1] On VR hand overlap, switch state
  (bind _asvrtemplate_game_mode (cast `/Game/SjolieVRTemplates/VRTemplateGameMode` (`GameplayStatics.GetGameMode`)))
  (bind _result (`/Game/SjolieVRTemplates/VRTemplateGameMode.IsVRHand` _asvrtemplate_game_mode OtherActor))
  (if _result
    (bind _output_get (set `self.TurnedOn` (not (`self.TurnedOn`))))
    ;[1 1 1] And play sound
    (`GameplayStatics.PlaySoundAtLocation` (select `bool` _output_get :`false` "/Game/VeaR/Sounds/SFX/ButtonOff.ButtonOff" :`true` "/Game/VeaR/Sounds/SFX/ButtonOn.ButtonOn" :!type "SoundBase Object Reference") (`self.K2_GetActorLocation`) (struct) 1.0 1.0 0.0 null null null)
    ;[1 1 1] And callback
    (`/Game/VeaR/Geometry/Logic/BoolCallback.Callback` (`self.ButtonCallback`) (`self.TurnedOn`))))

(event `self.ReceiveTick`
  (params (DeltaSeconds :type "Float (single-precision)"))
  (bind _clone (`self.Clone`))
  (bind _buttoncolor (`self.ButtonColor`))
  ;[1 1 1] Set button color and emissiveness
  (`MaterialInstanceDynamic.SetVectorParameterValue` (`self.MaterialInstance`) "Color" _buttoncolor)
  (`MaterialInstanceDynamic.SetVectorParameterValue` (`self.MaterialInstance`) "EmissiveColor" (select `bool` (`self.TurnedOn`) :`true` _buttoncolor))
  ;[1 1 1] Synchronize clone state
  (`/Engine/EditorBlueprintResources/StandardMacros.IsValid` _clone
    (:`Is Valid`
      (set `/Game/VeaR/Geometry/BP_SmallButton.TurnedOn` (`self.TurnedOn`) _clone))))

(fn `UserConstructionScript`
  (`TextRenderComponent.K2_SetText` (`self.Label`) (`self.LabelText`)))