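; BP_Baby is a scripted baby prop actor that rises and levitates with gore and crying audio when its Animation event is called.
; The event plays the gore sound while the TL_MoveToLamp timeline drives the Baby component's absolute world Z.
; On completion, it plays the cry cue and starts TL_Levitate, which adds its curve value scaled by LevitateFactor to the current height on each update.
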(event `self.ReceiveBeginPlay`)

(event `Animation`
  (bind _baby (`self.Baby`))
  (bind _baby_2 (`self.Baby`))
  (bind (_returnvalue_x _returnvalue_y _returnvalue_z) (`KismetMathLibrary.BreakVector` (`SceneComponent.K2_GetComponentLocation` _baby)))
  (bind (_returnvalue_x_2 _returnvalue_y_2) (`KismetMathLibrary.BreakVector` (`SceneComponent.K2_GetComponentLocation` _baby_2)))
  (`AudioComponent.Play` (`self.SFX_Gore`) 0.0)
  (bind (_direction _z) (`Timeline|TL_MoveToLamp`)
    (:`Update`
      (`SceneComponent.K2_SetWorldLocation` _baby_2 (`KismetMathLibrary.MakeVector` _returnvalue_x_2 _returnvalue_y_2 _z) false true))
    (:`Finished`
      (`AudioComponent.Play` (`self.SFX_BabyCry_Cue`) 0.0)
      (bind (_direction_2 _z_2) (`Timeline|TL_Levitate`)
        (:`Update`
          (`SceneComponent.K2_SetWorldLocation` _baby (`KismetMathLibrary.MakeVector` _returnvalue_x _returnvalue_y (+ _returnvalue_z (* _z_2 (`self.LevitateFactor`)))) false true))))))

(fn `UserConstructionScript`)