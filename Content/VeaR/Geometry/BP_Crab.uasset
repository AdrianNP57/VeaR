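; BP_Crab is a hidden crab actor that drives a scripted finale ending in a return to the MainMenu level.
; VisualizeCrab reveals it, and MoveCrab dims every BP_Candle, plays a piano cry and starts AlphaTimeLine.
; Tick lerps the mesh from InitialTransform to FinalTransform using the timeline alpha.
; When the timeline finishes, a landing sound and quick camera fade precede a running-away sound and the level change.
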(event `self.ReceiveBeginPlay`
  (`SceneComponent.K2_SetRelativeTransform` (`self.SkeletalMesh`) (`self.InitialTransform`) false false)
  (`SceneComponent.SetVisibility` (`self.DefaultSceneRoot`) false true))

(event `self.ReceiveTick`
  (params (DeltaSeconds :type "Float (single-precision)"))
  ;[1 1 1] Interpolate transform
  (`SceneComponent.K2_SetRelativeTransform` (`self.SkeletalMesh`) (`KismetMathLibrary.TLerp` (`self.InitialTransform`) (`self.FinalTransform`) (stale `MoveCrab` _alpha)) false false))

(event `MoveCrab`
  (bind _outactors (`GameplayStatics.GetAllActorsOfClass` "/Game/VeaR/Geometry/BP_Candle.BP_Candle_C"))
  (for _array_element _outactors
    (set `/Game/VeaR/Geometry/BP_Candle.CurrentCandleIntensity` (* (`/Game/VeaR/Geometry/BP_Candle.CurrentCandleIntensity` _array_element) 0.35) _array_element))
  (`AudioComponent.Play` (`self.SFX_PianoCry`) 0.0)
  (bind (_direction _alpha) (`Timeline|AlphaTimeLine`)
    (:`Finished`
      (`AudioComponent.Play` (`self.SFX_Landing`) 0.0)
      (`PlayerCameraManager.StartCameraFade` :`self` (`GameplayStatics.GetPlayerCameraManager` 0) :`ToAlpha` 1.0 :`Duration` 0.1 :`bHoldWhenFinished` true)
      (`KismetSystemLibrary.Delay` 1.0)
      (`AudioComponent.Play` (`self.SFX_RunningAway`) 0.0)
      (`KismetSystemLibrary.Delay` 5.0)
      (`GameplayStatics.OpenLevel` "MainMenu"))))

(event `VisualizeCrab`
  (`SceneComponent.SetVisibility` (`self.DefaultSceneRoot`) true true))

(fn `UserConstructionScript`)